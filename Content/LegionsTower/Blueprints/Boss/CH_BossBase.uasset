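; Base boss character for Legions Tower, providing shared stats, melee attack and skill selection.
; On BeginPlay, StatsModifier applies SkillValue entries to health, armor, resist, damage and walk speed, then applies multipliers and fills current health.
; Resist ends at zero because its multiplier node is unused.
; DoBasicAttack toggles melee collision, SetRandomSkill picks a random skill index, and ReceiveDamage is an empty stub.
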(event EventBeginPlay
  (CallFunction|StatsModifier))

(event Collision|EventActorBeginOverlap
  (params (OtherActor :type Actor%20Object%20Reference)))

(event EventTick
  (params (DeltaSeconds :type Float%20%28single-precision%29)))

(fn ConstructionScript)

(fn DoBasicAttack
  (params (isAttacking :type Boolean))
  (bind _meleecollision (Variables|Default|GetMeleeCollision))
  (if isAttacking
    (Collision|SetCollisionEnabled _meleecollision "QueryOnly")
    (else
      (Collision|SetCollisionEnabled _meleecollision "NoCollision")
      (Variables|Default|SetisAttacking false))))

(fn ReceiveDamage
  (params (DamageReceiving :type Float%20%28single-precision%29)))

(fn SetRandomSkill
  (Variables|Default|SetskillUsing (Math|Random|RandomIntegerinRange 0 (- (Variables|Default|GetnumberOfSkills) 1))))

(fn StatsModifier
  (bind _charactermovement (Variables|Character|GetCharacterMovement))
  (for _array_element (Variables|Default|GetskillValue)
    (switch Utilities|FlowControl|Switch|SwitchonE_SkillNames (.skillname _array_element)
      (:NewEnumerator8
        (Variables|Default|SetmaxHealth (+ (.amount _array_element) (Variables|Default|GetmaxHealth))))
      (:NewEnumerator9
        (Variables|Default|SetmaxHealth (- (Variables|Default|GetmaxHealth) (.amount _array_element))))
      (:NewEnumerator3
        (Variables|Default|Setresist (+ (Variables|Default|Getresist) (.amount _array_element))))
      (:NewEnumerator4
        (Variables|Default|Setresist (- (Variables|Default|Getresist) (.amount _array_element))))
      (:NewEnumerator5
        (Variables|Default|Setarmor (+ (Variables|Default|Getarmor) (.amount _array_element))))
      (:NewEnumerator6
        (Variables|Default|Setarmor (- (Variables|Default|Getarmor) (.amount _array_element))))
      (:NewEnumerator1
        (Variables|/Script/Engine.CharacterMovementComponent|SetMaxWalkSpeed _charactermovement (+ (Variables|/Script/Engine.CharacterMovementComponent|GetMaxWalkSpeed _charactermovement) (.amount _array_element))))
      (:NewEnumerator2
        (Variables|/Script/Engine.CharacterMovementComponent|SetMaxWalkSpeed _charactermovement (- (Variables|/Script/Engine.CharacterMovementComponent|GetMaxWalkSpeed _charactermovement) (.amount _array_element))))
      (:NewEnumerator0
        (Variables|Default|Setdamage (+ (Variables|Default|Getdamage) (.amount _array_element))))
      (:NewEnumerator7
        (Variables|Default|Setdamage (- (Variables|Default|Getdamage) (.amount _array_element))))
      (:NewEnumerator12
        (LocalVariables|SetDamageMultiplier (.amount _array_element)))
      (:NewEnumerator13
        (LocalVariables|SetArmorMultiplier (.amount _array_element)))
      (:NewEnumerator14
        (LocalVariables|SetResistMultiplier (.amount _array_element)))
      (:NewEnumerator15
        (LocalVariables|SetHealthMultiplier (.amount _array_element)))))
  (Variables|Default|Setarmor (* (Variables|Default|Getarmor) (LocalVariables|GetArmorMultiplier)))
  (Variables|Default|Setresist 0.0)
  (Variables|Default|Setdamage (* (Variables|Default|Getdamage) (LocalVariables|GetDamageMultiplier)))
  (bind _output_get (Variables|Default|SetmaxHealth (* (Variables|Default|GetmaxHealth) (LocalVariables|GetHealthMultiplier))))
  (Variables|Default|SetcurrentHealth _output_get))