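; Greg, an easy-tier boss for Legions Tower with a collision-based skill that deals non-physical damage to the player character.
; UseSkill checks casting state, disables mesh collision, plays a montage and writes its length to the Blackboard as skill time.
; DoSkillOne toggles the skill hitbox, whose overlaps during casting deal random damage from a configured range.
; The logic restoring mesh collision and clearing IsCasting is unconnected here.
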(event OnComponentBeginOverlap(SkillOneCollision)
  (params (OverlappedComponent :type Primitive%20Component%20Object%20Reference) (OtherActor :type Actor%20Object%20Reference) (OtherComp :type Primitive%20Component%20Object%20Reference) (OtherBodyIndex :type Integer) (bFromSweep :type Boolean) (SweepResult :type Hit%20Result%20Structure%20%28by%20ref%29))
  (if (Variables|Default|GetisCasting)
    (bind _asthird_person_character (Utilities|Casting|CastToThirdPersonCharacter OtherActor))
    (Default|ReceivingDamage _asthird_person_character (CallFunction|FGetRandomDamagefromArrayRange (Variables|Default|GetSkill1Damage)) false)))

(event EventBeginPlay
  (|CallParentFunction) ; This node is disabled and will not be called.\nDrag off pins to build functionality.
)

(event Collision|EventActorBeginOverlap
  (params (OtherActor :type Actor%20Object%20Reference))
  (|CallParentFunction OtherActor) ; This node is disabled and will not be called.\nDrag off pins to build functionality.
)

(event EventTick
  (params (DeltaSeconds :type Float%20%28single-precision%29))
  (|CallParentFunction DeltaSeconds) ; This node is disabled and will not be called.\nDrag off pins to build functionality.
)

(event EventUseSkill
  (if (Variables|Default|GetcanUseSkills?)
    (if (not (Variables|Default|GetisCasting))
      (switch int (Variables|Default|GetUsingSkillNumber)
        (:0
          (Variables|Default|SetisCasting true)
          (Variables|Default|SetCurrentLocation (Transformation|GetActorLocation))
          (Collision|SetCollisionEnabled (Variables|Character|GetMesh) "NoCollision")
          (bind _returnvalue (Animation|Montage|MontagePlay (Components|SkeletalMesh|GetAnimInstance (Variables|Character|GetMesh)) 0 1.0 "MontageLength" 0.0 true))
          (bind _output_get (Variables|Default|SetSkillTime _returnvalue))
          (AI|Components|Blackboard|SetValueasFloat (AI|GetBlackboard 0) (Variables|Default|GetSkillTimeName) _output_get))))))

(fn ConstructionScript
  (|CallParentFunction))

(fn DoSkillOne
  (params (IsAttacking? :type Boolean))
  (bind _skillonecollision (Variables|Default|GetSkillOneCollision))
  (if IsAttacking?
    (Collision|SetCollisionEnabled _skillonecollision "QueryOnly")
    (else
      (Collision|SetCollisionEnabled _skillonecollision "NoCollision"))))