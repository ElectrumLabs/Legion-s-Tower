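; Easy-tier Warrior boss that damages the player with a melee basic attack.
; Attack and CastSkill events only set the IsAttacking and IsCasting flags.
; When MeleeCollision overlaps a ThirdPersonCharacter, it applies Damage through ReceivingDamage, prints a debug message and calls DoBasicAttack with false.
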(event OnComponentBeginOverlap(MeleeCollision)
  (params (OverlappedComponent :type Primitive%20Component%20Object%20Reference) (OtherActor :type Actor%20Object%20Reference) (OtherComp :type Primitive%20Component%20Object%20Reference) (OtherBodyIndex :type Integer) (bFromSweep :type Boolean) (SweepResult :type Hit%20Result%20Structure%20%28by%20ref%29))
  ;[1 1 1] Basic Attack Collision
  (bind _asthird_person_character (Utilities|Casting|CastToThirdPersonCharacter OtherActor))
  (Default|ReceivingDamage _asthird_person_character (Variables|Default|Getdamage))
  (Development|PrintString "You received damage")
  (CallFunction|DoBasicAttack false))

(event EventBeginPlay
  (|CallParentFunction) ; This node is disabled and will not be called.\nDrag off pins to build functionality.
)

(event Collision|EventActorBeginOverlap
  (params (OtherActor :type Actor%20Object%20Reference))
  (|CallParentFunction OtherActor) ; This node is disabled and will not be called.\nDrag off pins to build functionality.
)

(event EventTick
  (params (DeltaSeconds :type Float%20%28single-precision%29))
  (|CallParentFunction DeltaSeconds) ; This node is disabled and will not be called.\nDrag off pins to build functionality.
)

(event EventAttack
  ;[1 1 1] Basic Attack
  (Variables|Default|SetisAttacking true))

(event EventCastSkill
  ;[1 1 1] Casting Skill
  (Variables|Default|SetisCasting true))

(fn ConstructionScript
  (|CallParentFunction))