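; Base boss character Blueprint holding shared combat stats and helpers.
; On BeginPlay it sets walk speed, then StatsModifier folds a SkillValue list of increases, decreases and multipliers into health, armor, resist, damage and speed.
; ReceivingDamage subtracts flat Armor or Resist by damage type, then updates the IsDead flag.
; Helpers toggle melee collision for attacks, pick a random skill index and roll damage within a range.
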(event EventBeginPlay
  (Variables|/Script/Engine.CharacterMovementComponent|SetMaxWalkSpeed (Variables|Character|GetCharacterMovement) (Variables|Attribute|GetBaseMovementSpeed))
  (CallFunction|StatsModifier))

(event Collision|EventActorBeginOverlap
  (params (OtherActor :type Actor%20Object%20Reference)))

(event EventTick
  (params (DeltaSeconds :type Float%20%28single-precision%29)))

(fn ConstructionScript)

(fn DoBasicAttack
  (params (isAttacking :type Boolean))
  (bind _meleecollision (Variables|Default|GetMeleeCollision))
  (if isAttacking
    ;[1 1 1] Enables collision when attacking.
    (Collision|SetCollisionEnabled _meleecollision "QueryOnly")
    (else
      ;[1 1 1] Disable collision after end of actionframe or has been hit
      (Collision|SetCollisionEnabled _meleecollision "NoCollision"))))

(fn ReceivingDamage
  (params (DamageReceiving :type Float%20%28single-precision%29) (isPhysicalDamage :type Boolean))
  (if isPhysicalDamage
    ;[1 1 1] Receiving Physical Damage
    (bind _output_get (LocalVariables|SetNewDamageOutput (- DamageReceiving (Variables|Attribute|GetArmor))))
    (if (>= _output_get 0.0)
      (Variables|Attribute|SetCurrentHealth (- (Variables|Attribute|GetCurrentHealth) _output_get))
      (CallFunction|CheckifDead))
    (else
      ;[1 1 1] Receiving Resist Damage
      (bind _output_get_2 (LocalVariables|SetNewDamageOutput (- DamageReceiving (Variables|Attribute|GetResist))))
      (if (>= _output_get_2 0.0)
        (Variables|Attribute|SetCurrentHealth (- (Variables|Attribute|GetCurrentHealth) _output_get_2))
        (CallFunction|CheckifDead)))))

(fn SetRandomSkill
  (Variables|Core|SetUsingSkillNumber (Math|Random|RandomIntegerinRange 0 (- (Variables|Attribute|GetNumberOfSkills) 1))))

(fn StatsModifier
  (bind _charactermovement (Variables|Character|GetCharacterMovement))
  (for _array_element (Variables|Attribute|GetSkillValue)
    (switch Utilities|FlowControl|Switch|SwitchonE_SkillNames (.skillname _array_element)
      (:NewEnumerator8
        ;[1 1 1] Increase / Decrease Health
        (Variables|Attribute|SetMaxHealth (+ (.amount _array_element) (Variables|Attribute|GetMaxHealth))))
      (:NewEnumerator9
        (Variables|Attribute|SetMaxHealth (- (Variables|Attribute|GetMaxHealth) (.amount _array_element))))
      (:NewEnumerator3
        ;[1 1 1] Increase / Decrease Resist
        (Variables|Attribute|SetResist (+ (Variables|Attribute|GetResist) (.amount _array_element))))
      (:NewEnumerator4
        (Variables|Attribute|SetResist (- (Variables|Attribute|GetResist) (.amount _array_element))))
      (:NewEnumerator5
        ;[1 1 1] Increase / Decrease Armor
        (Variables|Attribute|SetArmor (+ (Variables|Attribute|GetArmor) (.amount _array_element))))
      (:NewEnumerator6
        (Variables|Attribute|SetArmor (- (Variables|Attribute|GetArmor) (.amount _array_element))))
      (:NewEnumerator1
        ;[1 1 1] Increase / Decreate Movement Speed
        (Variables|/Script/Engine.CharacterMovementComponent|SetMaxWalkSpeed _charactermovement (+ (Variables|/Script/Engine.CharacterMovementComponent|GetMaxWalkSpeed _charactermovement) (.amount _array_element))))
      (:NewEnumerator2
        (Variables|/Script/Engine.CharacterMovementComponent|SetMaxWalkSpeed _charactermovement (- (Variables|/Script/Engine.CharacterMovementComponent|GetMaxWalkSpeed _charactermovement) (.amount _array_element))))
      (:NewEnumerator0
        ;[1 1 1] Increase / Decrease Damage
        (Variables|Attribute|SetDamage (Utilities|Struct|MakeS_DamageRange (+ (.minimumdamage (Variables|Attribute|GetDamage)) (.amount _array_element)) (+ (.maximumdamage (Variables|Attribute|GetDamage)) (.amount _array_element)))))
      (:NewEnumerator7
        (Variables|Attribute|SetDamage (Utilities|Struct|MakeS_DamageRange (- (.minimumdamage (Variables|Attribute|GetDamage)) (.amount _array_element)) (- (.maximumdamage (Variables|Attribute|GetDamage)) (.amount _array_element)))))
      (:NewEnumerator12
        ;[1 1 1] Set Damage Multiplier
        (LocalVariables|SetDamageMultiplier (.amount _array_element)))
      (:NewEnumerator13
        ;[1 1 1] Set Armor Multiplier
        (LocalVariables|SetArmorMultiplier (.amount _array_element)))
      (:NewEnumerator14
        ;[1 1 1] Set Resist Multiplier
        (LocalVariables|SetResistMultiplier (.amount _array_element)))
      (:NewEnumerator15
        ;[1 1 1] Set Health Multiplier
        (LocalVariables|SetHealthMultiplier (.amount _array_element)))))
  ;[1 1 1] Finalize Stats
  (Variables|Attribute|SetArmor (* (Variables|Attribute|GetArmor) (LocalVariables|GetArmorMultiplier)))
  (Variables|Attribute|SetResist (* (Variables|Attribute|GetResist) (LocalVariables|GetResistMultiplier)))
  (Variables|Attribute|SetDamage (Utilities|Struct|MakeS_DamageRange (* (.minimumdamage (Variables|Attribute|GetDamage)) (LocalVariables|GetDamageMultiplier)) (* (.maximumdamage (Variables|Attribute|GetDamage)) (LocalVariables|GetDamageMultiplier))))
  (bind _output_get (Variables|Attribute|SetMaxHealth (* (Variables|Attribute|GetMaxHealth) (LocalVariables|GetHealthMultiplier))))
  (Variables|Attribute|SetCurrentHealth _output_get))

(fn FGetRandomDamagefromArrayRange
  (params (SkillDamage :type S%20Damage%20Range%20Structure))
  (bind (_minimumdamage _maximumdamage) (Utilities|Struct|BreakS_DamageRange SkillDamage))
  (return (Math|Random|RandomFloatinRange _minimumdamage _maximumdamage)))

(fn CheckifDead
  (if (<= (Variables|Attribute|GetCurrentHealth) 0.0)
    (Variables|Core|SetisDead true)
    (else
      (Variables|Core|SetisDead false))))