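; BP_ProxySwordHitbox is a short-lived sword slash hitbox that damages bosses.
; On spawn, a Slash timeline sweeps its yaw from the starting rotation, and the actor destroys itself when the timeline finishes.
; Each tick it snaps to its owner's location, so the swing follows the wielder.
; Any overlapping BP_BaseBoss receives fixed physical damage through ReceivingDamage.
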(event EventBeginPlay
  (Variables|Default|SetOriginalRotation (Transformation|GetActorRotation))
  (bind _newtrack_0 (Timeline|Slash Play)
    (:Update
      (Transformation|SetActorRotation (Math|Rotator|MakeRotator (.roll (Variables|Default|GetOriginalRotation)) (.pitch (Variables|Default|GetOriginalRotation)) (+ (.yaw (Variables|Default|GetOriginalRotation)) _newtrack_0))))
    (:Finished
      (Actor|DestroyActor))))

(event EventTick
  (params (DeltaSeconds :type Float%20%28single-precision%29))
  (Transformation|SetActorLocation (Transformation|GetActorLocation (Components|GetOwner)) false false))

(event Collision|EventActorBeginOverlap
  (params (OtherActor :type Actor%20Object%20Reference))
  (bind _asbp_base_boss (Utilities|Casting|CastToBP_BaseBoss OtherActor))
  (Default|ReceivingDamage _asbp_base_boss 1e+01 true))

(fn ConstructionScript)