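; NPC_Priest is a priest NPC in the RestFloor area of LegionsTower that brings up a priest HUD when the player is in range.
; A Sphere component's begin overlap checks for a ThirdPersonCharacter and calls ShowPriestHUD on the TowerPC controller of player 0.
; End overlap calls HideStoreHUD on that controller rather than a priest-specific hide function.
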(event OnComponentBeginOverlap(Sphere)
  (params (OverlappedComponent :type Primitive%20Component%20Object%20Reference) (OtherActor :type Actor%20Object%20Reference) (OtherComp :type Primitive%20Component%20Object%20Reference) (OtherBodyIndex :type Integer) (bFromSweep :type Boolean) (SweepResult :type Hit%20Result%20Structure%20%28by%20ref%29))
  ;[1 1 1] Show HUD when player is in range
  (Utilities|Casting|CastToThirdPersonCharacter OtherActor)
  (bind _astower_pc (Utilities|Casting|CastToTowerPC (Game|GetPlayerController 0)))
  (Default|ShowPriestHUD _astower_pc))

(event OnComponentEndOverlap(Sphere)
  (params (OverlappedComponent :type Primitive%20Component%20Object%20Reference) (OtherActor :type Actor%20Object%20Reference) (OtherComp :type Primitive%20Component%20Object%20Reference) (OtherBodyIndex :type Integer))
  (Utilities|Casting|CastToThirdPersonCharacter OtherActor)
  (bind _astower_pc (Utilities|Casting|CastToTowerPC (Game|GetPlayerController 0)))
  (Default|HideStoreHUD _astower_pc))

(event EventBeginPlay
  (|CallParentFunction) ; This node is disabled and will not be called.\nDrag off pins to build functionality.
)

(event Collision|EventActorBeginOverlap
  (params (OtherActor :type Actor%20Object%20Reference))
  (|CallParentFunction OtherActor) ; This node is disabled and will not be called.\nDrag off pins to build functionality.
)

(event EventTick
  (params (DeltaSeconds :type Float%20%28single-precision%29))
  (|CallParentFunction DeltaSeconds) ; This node is disabled and will not be called.\nDrag off pins to build functionality.
)

(fn ConstructionScript
  (|CallParentFunction))