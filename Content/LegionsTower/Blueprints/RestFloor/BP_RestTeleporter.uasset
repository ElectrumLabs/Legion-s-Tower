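; BP_RestTeleporter is the rest floor exit that sends the player on to a random level.
; On BeginPlay it caches the tower game instance, rest game mode and tower player controller.
; When the player character overlaps its box, it saves the character's stats and the controller's equipment and consumables to the game instance.
; The game instance then opens the random level, with the saved data held across the transition.
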(event OnComponentBeginOverlap(Box)
  (params (OverlappedComponent :type Primitive%20Component%20Object%20Reference) (OtherActor :type Actor%20Object%20Reference) (OtherComp :type Primitive%20Component%20Object%20Reference) (OtherBodyIndex :type Integer) (bFromSweep :type Boolean) (SweepResult :type Hit%20Result%20Structure%20%28by%20ref%29))
  (bind _playerpc (Variables|Default|GetPlayerPC))
  (bind _asthird_person_character (Utilities|Casting|CastToThirdPersonCharacter OtherActor))
  (Default|SaveData (Variables|Default|GetGameInstanceREF) (Variables|/Game/LegionsTower/Blueprints/Character/ThirdPersonCharacter.ThirdPersonCharacter_C|GetHealth _asthird_person_character) (Variables|/Game/LegionsTower/Blueprints/Character/ThirdPersonCharacter.ThirdPersonCharacter_C|GetArmor _asthird_person_character) (Variables|/Game/LegionsTower/Blueprints/Character/ThirdPersonCharacter.ThirdPersonCharacter_C|GetResist _asthird_person_character) (Variables|/Game/LegionsTower/Blueprints/Character/ThirdPersonCharacter.ThirdPersonCharacter_C|GetStamina _asthird_person_character) (Utilities|Struct|MakeS_Inventory (Variables|/Game/LegionsTower/Blueprints/Core/TowerPC.TowerPC_C|GetCurrentWeapon _playerpc) (Variables|/Game/LegionsTower/Blueprints/Core/TowerPC.TowerPC_C|GetCurrentUpperArmor _playerpc) (Variables|/Game/LegionsTower/Blueprints/Core/TowerPC.TowerPC_C|GetCurrentLowerArmor _playerpc) (Variables|/Game/LegionsTower/Blueprints/Core/TowerPC.TowerPC_C|GetConsumable _playerpc)))
  (Default|OpenRandomLevel (Variables|Default|GetGameInstanceREF)))

(event EventBeginPlay
  (Utilities|FlowControl|Sequence
    (:then_0
      (bind _astower_game_instance (Utilities|Casting|CastToTowerGameInstance (Game|GetGameInstance)))
      (Variables|Default|SetGameInstanceREF _astower_game_instance))
    (:then_1
      (bind _asrest_game_mode (Utilities|Casting|CastToRestGameMode (Game|GetGameMode)))
      (Variables|Default|SetGameModeREF _asrest_game_mode))
    (:then_2
      (bind _astower_pc (Utilities|Casting|CastToTowerPC (Game|GetPlayerController 0)))
      (Variables|Default|SetPlayerPC _astower_pc))))

(fn ConstructionScript)