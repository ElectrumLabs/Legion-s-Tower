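; Game instance for the tower game that holds player and run state, including floor level, gold, stats, inventory and consumables.
; SaveData stores health, armor, resist and stamina, while FReturnPlayerStats hands back health, stamina and inventory.
; AddConsumable appends to the consumable list, and ResetData zeroes only floor, gold and current health.
; It also opens levels by name or picks one at random from a map name list.
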(event Custom|AddConsumable
  (params (NewItem :type S%20Consumable%20Structure))
  ;[1 1 1] Add Item
  (Utilities|Array|Add (Variables|Default|GetConsumable) NewItem))

(fn ResetData
  (Variables|Default|SetFloorLevel 0)
  (Variables|Default|SetGold 0)
  (Variables|Player'sStat|SetCurrentHealth 0.0))

(fn FReturnPlayerStats
  (return (Variables|Player'sStat|GetCurrentHealth) (Variables|Player'sStat|GetMaximumHealth) (Variables|Player'sStat|GetCurrentStamina) (Variables|Player'sStat|GetMaximumStamina) (Variables|Player'sStat|GetInventory)))

(fn OpenRandomLevel
  (bind _levelmapnames (Variables|Default|GetLevelMapNames))
  (Game|OpenLevel(byName) (Utilities|Array|Get(acopy) _levelmapnames (Math|Random|RandomIntegerinRange 0 (- (Utilities|Array|Length _levelmapnames) 1)))))

(fn OpenLevel
  (params (Level%20Name :type Name))
  (Game|OpenLevel(byName) Level%20Name))

(fn SaveData
  (params (CurrentHealth :type Float%20%28single-precision%29) (Armor :type Float%20%28single-precision%29) (Resist :type Float%20%28single-precision%29) (CurrentStamina :type Float%20%28single-precision%29))
  (Variables|Player'sStat|SetCurrentHealth CurrentHealth)
  (Variables|Player'sStat|SetArmor Armor)
  (Variables|Player'sStat|SetResist Resist)
  (Variables|Player'sStat|SetCurrentStamina CurrentStamina))