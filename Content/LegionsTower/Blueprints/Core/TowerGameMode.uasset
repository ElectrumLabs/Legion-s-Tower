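; Game mode for a tower floor that sets up the player and a boss when play begins.
; BeginPlay caches the TowerGameInstance, loads its saved inventory into TowerPC, then spawns the ThirdPersonCharacter with that instance's health and stamina.
; It picks and spawns a random boss from the easy list on lower floors.
; Higher floors only print a placeholder message, leaving the boss class unset by SetBoss.
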(event Custom|SpawnPlayerFromGameInstance
  (bind _gameinstanceref (Variables|Default|GetGameInstanceREF))
  (bind (_currenthealth _maximumhealth _currentstamina _maximumstamina) (Default|FReturnPlayerStats _gameinstanceref))
  (Game|SpawnActorfromClass "/Game/LegionsTower/Blueprints/Character/ThirdPersonCharacter.ThirdPersonCharacter_C" (Math|Transform|MakeTransform "0, 0, 0" "0, 0, 0" "1,1,1") "Undefined" 0 _currenthealth _maximumhealth _currentstamina _maximumstamina 0))

(event Custom|LoadPlayerInventory
  (bind _astower_pc (Utilities|Casting|CastToTowerPC (Game|GetPlayerController 0)))
  (Default|LoadInventory _astower_pc (Variables|/Game/LegionsTower/Blueprints/Core/TowerGameInstance.TowerGameInstance_C|GetInventory (Variables|Default|GetGameInstanceREF))))

(event Custom|SpawnBoss
  (Game|SpawnActorfromClass (Variables|Default|GetBossToSpawn) (Math|Transform|MakeTransform "500.000000, 0,100.000000" "0, 0, 0" "1,1,1") "AdjustIfPossibleButAlwaysSpawn" 0 0))

(event Custom|SetBoss
  (bind _gameinstanceref (Variables|Default|GetGameInstanceREF))
  (bind _easylevelbosses (Variables|/Game/LegionsTower/Blueprints/Core/TowerGameInstance.TowerGameInstance_C|GetEasyLevelBosses _gameinstanceref))
  (bind _returnvalue (Utilities|Array|Length _easylevelbosses))
  (bind _returnvalue_2 (- _returnvalue 1))
  (bind _returnvalue_3 (Math|Random|RandomIntegerinRange 0 _returnvalue_2))
  ;[1 1 1] Set the boss for the floor
  (if (< (Variables|/Game/LegionsTower/Blueprints/Core/TowerGameInstance.TowerGameInstance_C|GetFloorLevel _gameinstanceref) 9)
    (Variables|Default|SetBossToSpawn (Utilities|Array|Get(acopy) _easylevelbosses _returnvalue_3))
    (Development|PrintString (Utilities|String|ToString(Integer) _returnvalue_3))
    (else
      (Development|PrintString "int boss function"))))

(event EventBeginPlay
  (Utilities|FlowControl|Sequence
    (:then_0
      (bind _astower_game_instance (Utilities|Casting|CastToTowerGameInstance (Game|GetGameInstance)))
      (Variables|Default|SetGameInstanceREF _astower_game_instance))
    (:then_1
      (CallFunction|LoadPlayerInventory))
    (:then_2
      (CallFunction|SpawnPlayerfromGameInstance))
    (:then_3
      (CallFunction|SetBoss))
    (:then_4
      (CallFunction|SpawnBoss))))

(event EventTick
  (params (DeltaSeconds :type Float%20%28single-precision%29)))

(fn ConstructionScript)