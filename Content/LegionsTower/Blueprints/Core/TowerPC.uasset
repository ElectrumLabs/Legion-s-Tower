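; Player controller for LegionsTower that owns the player HUD, the merchant and priest store screens, and the consumable inventory.
; BeginPlay caches the player state and creates the HUD; store widgets are created on first use, then toggled by visibility while switching input modes.
; The Consumable input uses the first inventory item, applying a flat health or stamina restore to the character and removing it.
; Dialogue events show or hide text on the HUD.
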(event Custom|AddConsumable
  (params (NewItem :type S%20Consumable%20Structure%20%28by%20ref%29))
  ;[1 1 1] Add consumable to inventory
  (Utilities|Array|Add (Variables|Default|GetConsumable) NewItem))

(event EventBeginPlay
  (Utilities|FlowControl|Sequence
    (:then_0
      (bind _astower_player_state (Utilities|Casting|CastToTowerPlayerState (Variables|GetPlayerState)))
      (Variables|Default|SetPlayerStateREF _astower_player_state))
    (:then_1
      (CallFunction|ShowPlayerHUD))))

(event Input|ActionEvents|InputActionConsumable
  (params (Key :type Key%20Structure))
  (bind _returnvalue (Game|Player|GetPlayerPawn 0))
  (bind _consumable (Variables|Default|GetConsumable))
  (bind _consumable_2 (Variables|Default|GetConsumable))
  (bind _asthird_person_character (Utilities|Casting|CastToThirdPersonCharacter _returnvalue))
  (bind _output (Utilities|Array|Get(acopy) _consumable))
  (bind _output_2 (Utilities|Array|Get(acopy) _consumable_2))
  (bind _effectvalue (Utilities|Struct|BreakS_Consumable _output))
  (bind (_itemid _itemtier _itemname _itemdescription _goldvalue _effect) (Utilities|Struct|BreakS_Consumable _output_2))
  ;[1 1 1] Check if the player has at least one consumable
  (:Pressed
    (if (Utilities|Array|IsValidIndex (Variables|Default|GetConsumable))
      (Development|PrintString (Utilities|String|ToString(Text) _itemname))
      (switch Utilities|FlowControl|Switch|SwitchonE_ConsumableEffect _effect
        (:NewEnumerator0
          ;[1 1 1] Add a flat amount of health to the character
          (Default|HealHealth _asthird_person_character _effectvalue))
        (:NewEnumerator1
          ;[1 1 1] Add a flat amount of stamina to the character
          (Default|ReplenishStamina _asthird_person_character _effectvalue)))
      (Utilities|Array|RemoveIndex (Variables|Default|GetConsumable)))))

(event Custom|ShowMerchantHUD
  ;[1 1 1] Show the store HUD
  (Utilities|IsValid (Variables|Default|GetMerchantStoreREF)
    (:Is%20Valid
      (Widget|SetVisibility (Variables|Default|GetMerchantStoreREF) "Visible"))
    (:Is%20Not%20Valid
      (bind _returnvalue (UserInterface|CreateWidget "/Game/LegionsTower/Blueprints/RestFloor/Widgets/WBP_MerchantStore.WBP_MerchantStore_C"))
      (Variables|Default|SetMerchantStoreREF _returnvalue)
      (UserInterface|Viewport|AddtoViewport (Variables|Default|GetMerchantStoreREF) 0)))
  (Input|SetInputModeGameandUI self 0 "DoNotLock" true))

(event Custom|HideStoreHUD
  (bind _merchantstoreref (Variables|Default|GetMerchantStoreREF))
  (bind _prieststoreref (Variables|Default|GetPriestStoreREF))
  ;[1 1 1] Remove the store HUD
  (Utilities|FlowControl|Sequence
    (:then_0
      (Utilities|IsValid _merchantstoreref
        (:Is%20Valid
          (Widget|SetVisibility _merchantstoreref "Hidden"))))
    (:then_1
      (Utilities|IsValid _prieststoreref
        (:Is%20Valid
          (Widget|SetVisibility _prieststoreref "Hidden"))))
    (:then_2
      (Input|SetInputModeGameOnly self))))

(event Custom|ShowPlayerHUD
  (Utilities|IsValid (Variables|Default|GetPlayerHUDREF)
    (:Is%20Valid
      _)
    (:Is%20Not%20Valid
      (bind _returnvalue (UserInterface|CreateWidget "/Game/LegionsTower/Blueprints/Character/Widgets/WBP_PlayerHUD.WBP_PlayerHUD_C" 0 (.AsThird%20Person%20Character (Utilities|Casting|CastToThirdPersonCharacter (Pawn|GetControlledPawn)))))
      (Variables|Default|SetPlayerHUDREF _returnvalue)))
  (UserInterface|Viewport|AddtoViewport (Variables|Default|GetPlayerHUDREF) 0))

(event Custom|ShowPriestHUD
  ;[1 1 1] Show the merchant HUD
  (Utilities|IsValid (Variables|Default|GetPriestStoreREF)
    (:Is%20Valid
      (Widget|SetVisibility (Variables|Default|GetPriestStoreREF) "Visible"))
    (:Is%20Not%20Valid
      (bind _returnvalue (UserInterface|CreateWidget "/Game/LegionsTower/Blueprints/RestFloor/Widgets/WBP_PriestStore.WBP_PriestStore_C"))
      (Variables|Default|SetPriestStoreREF _returnvalue)
      (UserInterface|Viewport|AddtoViewport (Variables|Default|GetPriestStoreREF) 0)))
  (Input|SetInputModeGameandUI self 0 "DoNotLock" true))

(event Custom|UpdateDialogueText
  (params (DialogueText :type Text))
  (bind _playerhudref (Variables|Default|GetPlayerHUDREF))
  (Variables|/Game/LegionsTower/Blueprints/Character/Widgets/WBP_PlayerHUD.WBP_PlayerHUD_C|SetDialogueText _playerhudref DialogueText)
  (Widget|SetVisibility (Variables|/Game/LegionsTower/Blueprints/Character/Widgets/WBP_PlayerHUD.WBP_PlayerHUD_C|GetDTextBox _playerhudref) "Visible"))

(event Custom|HideDialogueText
  (Widget|SetVisibility (Variables|/Game/LegionsTower/Blueprints/Character/Widgets/WBP_PlayerHUD.WBP_PlayerHUD_C|GetDTextBox (Variables|Default|GetPlayerHUDREF)) "Collapsed"))

(fn ConstructionScript)